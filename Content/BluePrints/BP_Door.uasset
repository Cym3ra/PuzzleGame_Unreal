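; BP_Door is a door that swings open when its Interact event receives a BP_CheckPuzzleButton as the actor.
; The OpenCloseDoor timeline plays from the start, lerping the door's relative yaw from 180 to 80 degrees, with no reverse path.
; Each timeline update also plays OpenDoor_Cue at the location of the BP_MyCharacter cached on BeginPlay.
; An unconnected BP_LightPuzzle class check never runs.
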(event EventBeginPlay
  (bind _returnvalue (Actor|GetActorOfClass "/Game/BluePrints/BP_MyCharacter.BP_MyCharacter_C"))
  (Variables|Default|SetCharacter_REF _returnvalue))

(event EventInteract
  (params (Actor :type Actor%20Object%20Reference) (HitResult :type Hit%20Result%20Structure))
  (Utilities|Casting|CastToBP_CheckPuzzleButton Actor)
  (bind _doortrack (Timeline|Open/Close%20door PlayFromStart)
    (:Update
      (Transformation|SetRelativeRotation (Variables|Default|GetDoor) (Math|Rotator|MakeRotator 0.0 0.0 (Math|Float|Lerp 1.8e+02 8e+01 _doortrack)) false false)
      (Audio|PlaySoundatLocation "/Game/Audio/OpenDoor_Cue.OpenDoor_Cue" (Transformation|GetActorLocation (Variables|Default|GetCharacter_REF)) "0, 0, 0" 1.0 1.0 0.0 0 0 0 0))))

(fn ConstructionScript)