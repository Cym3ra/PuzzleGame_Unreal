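; Interactable button that checks a colour-code puzzle and opens an assigned door when the code is correct.
; On Interact it compares each puzzle piece's ColorIndex against ColorCode by array position.
; The first success runs a push-in timeline whose every update also plays the success cue and messages DoorToOpen through BPI_Interface.
; A wrong code resets all pieces to index 0, refreshes their lights and plays an error cue per piece.
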(event EventBeginPlay
  (bind _returnvalue (Actor|GetActorOfClass "/Game/BluePrints/BP_MyCharacter.BP_MyCharacter_C"))
  (Variables|Default|SetCharacter_REF _returnvalue))

(event Collision|EventActorBeginOverlap
  (params (OtherActor :type Actor%20Object%20Reference)))

(event EventTick
  (params (DeltaSeconds :type Float%20%28single-precision%29)))

(event EventInteract
  (params (Actor :type Actor%20Object%20Reference) (HitResult :type Hit%20Result%20Structure))
  (Variables|Default|SetisCorrect? true)
  (bind (_array_element _array_index) (Utilities|Array|ForEachLoopwithBreak (Variables|Default|GetPuzzlePieces) :!label _label)
    (:LoopBody
      (if (!= (Variables|/Game/BluePrints/BP_LampSwitch.BP_LampSwitch_C|GetColorIndex _array_element) (Utilities|Array|Get(acopy) (Variables|Default|GetColorCode) _array_index))
        (Variables|Default|SetisCorrect? false)
        (goto _label Break)))
    (:Completed
      (if (Variables|Default|GetisCorrect?)
        ;[1 1 1] If color corresponds with the index given, it opens the door chosen in the viewport to open. First it makes the button push inwards to show it was correct, then uses the interact on the door BP
        (Utilities|FlowControl|DoOnce false
          (:Completed
            (bind _doortoopen (Variables|Default|GetDoorToOpen)
              (:then
                (if (Utilities|DoesObjectImplementInterface _doortoopen "/Game/BluePrints/BPI_Interface.BPI_Interface_C")
                  (bind _pushbutton (Timeline|ButtonPressDown PlayFromStart)
                    (:Update
                      (Transformation|SetRelativeLocation (Variables|Default|GetButton) _pushbutton false false)
                      (Audio|PlaySoundatLocation "/Game/Audio/Success_Cue.Success_Cue" (Transformation|GetActorLocation (Variables|Default|GetCharacter_REF)) "0, 0, 0" 1.0 1.0 0.0 0 0 0 0)
                      (Class|BPIInterface|Interact(Message) _doortoopen self)))))
              (:else))))
        (else
          ;[1 1 1] if color is not correct, sets the color of all back to white when button is pressed
          (for _array_element_2 (Variables|Default|GetPuzzlePieces)
            (Variables|/Game/BluePrints/BP_LampSwitch.BP_LampSwitch_C|SetColorIndex _array_element_2 0)
            (Default|UpdateLightColor _array_element_2)
            (Audio|PlaySoundatLocation "/Game/Audio/Error_Cue.Error_Cue" (Transformation|GetActorLocation (Variables|Default|GetCharacter_REF)) "0, 0, 0" 0.8 1.0 0.0 0 0 0 0)))))))

(fn ConstructionScript)