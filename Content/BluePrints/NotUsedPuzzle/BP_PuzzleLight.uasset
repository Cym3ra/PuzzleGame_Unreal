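; BP_PuzzleLight is a light puzzle controller that opens its door once the count matches the number of lamps in the level.
; AddTo and RemoveFrom adjust a counter that cannot be decremented below zero.
; AddTo compares the counter to a live count of BP_LampPuzzle actors and calls WinCondition on a match.
; WinCondition plays the WinOpenDoor timeline, which drives the Door's relative yaw.
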(event Custom|AddTo
  ;[1 1 1] Add until int == the amount of lights in the scene
  (Variables|Default|SetInt (+ (Variables|Default|GetInt) 1))
  (bind _outactors (Actor|GetAllActorsOfClass "/Game/BluePrints/NotUsedPuzzle/BP_LampPuzzle.BP_LampPuzzle_C"))
  (if (== (Utilities|Array|Length _outactors) (Variables|Default|GetInt))
    (CallFunction|WinCondition)))

(event Custom|WinCondition
  (bind _doortrack (Timeline|WinOpenDoor Play)
    (:Update
      (Transformation|SetRelativeRotation (Variables|Default|GetDoor) (Math|Rotator|MakeRotator 0.0 0.0 _doortrack) false false))))

(event Custom|RemoveFrom
  (if (> (Variables|Default|GetInt) 0)
    (Variables|Default|SetInt (- (Variables|Default|GetInt) 1))))

(fn ConstructionScript)