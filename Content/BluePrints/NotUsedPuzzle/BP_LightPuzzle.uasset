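; BP_LightPuzzle is an unfinished light puzzle actor, filed under NotUsedPuzzle, with red, green and blue lamps that respond to interaction.
; Interact reads the hit component's first tag to select the matching lamp, then calls SwitchColor.
; SwitchColor always sets that lamp to the same hardcoded red, with no cycling or solve check.
; ChangeColor only copies ColorList into ColorArray and is not called here.
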(event Custom|SwitchColor
  (Rendering|Components|Light|SetLightColor (Variables|Default|GetLighToChange) "(R=0.281250,G=0.000000,B=0.000000,A=1.000000)" true))

(event EventBeginPlay)

(event Collision|EventActorBeginOverlap
  (params (OtherActor :type Actor%20Object%20Reference)))

(event EventTick
  (params (DeltaSeconds :type Float%20%28single-precision%29)))

(event EventInteract
  (params (Actor :type Actor%20Object%20Reference) (HitResult :type Hit%20Result%20Structure))
  (switch name (Utilities|Array|Get(acopy) (Variables|/Script/Engine.ActorComponent|GetComponentTags (.HitComponent (Collision|BreakHitResult HitResult))))
    (:Blue
      (Variables|Default|SetLighToChange (Variables|Default|GetBlueLamp)))
    (:Red
      (Variables|Default|SetLighToChange (Variables|Default|GetRedLamp)))
    (:Green
      (Variables|Default|SetLighToChange (Variables|Default|GetGreenLamp))))
  (CallFunction|SwitchColor))

(fn ConstructionScript)

(fn ChangeColor
  (LocalVariables|SetColorArray (Variables|Default|GetColorList)))