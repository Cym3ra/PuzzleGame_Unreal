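; BP_LampPuzzle is one lamp in a color-matching puzzle, cycling its point light through blue, green and red on Interact.
; A box overlap enables player input only while in range, and the construction script applies the starting color.
; Matching LightOrderNumber adds to the tally on the first BP_PuzzleLight found in the level.
; Other colors subtract through a DoOnce that resets on each match, preventing repeated removals.
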(event OnComponentBeginOverlap(Box)
  (params (OverlappedComponent :type Primitive%20Component%20Object%20Reference) (OtherActor :type Actor%20Object%20Reference) (OtherComp :type Primitive%20Component%20Object%20Reference) (OtherBodyIndex :type Integer) (bFromSweep :type Boolean) (SweepResult :type Hit%20Result%20Structure%20%28by%20ref%29))
  (Input|EnableInput (Game|GetPlayerController 0)))

(event OnComponentEndOverlap(Box)
  (params (OverlappedComponent :type Primitive%20Component%20Object%20Reference) (OtherActor :type Actor%20Object%20Reference) (OtherComp :type Primitive%20Component%20Object%20Reference) (OtherBodyIndex :type Integer))
  (Input|DisableInput (Game|GetPlayerController 0)))

(event Custom|Remove
  ;[1 1 1] Removes on a do once so it doesnt counter out the other lights
  (Utilities|FlowControl|DoOnce false
    (:Completed
      (Default|Removefrom (Variables|Default|GetPuzzleLight_REF)))))

(event EventInteract
  (params (Actor :type Actor%20Object%20Reference) (HitResult :type Hit%20Result%20Structure))
  ;[1 1 1] Switching between colors, and if int == the order number it adds one to puzzles tally
  (Variables|Default|SetLightInt (+ (Variables|Default|GetLightInt) 1))
  (if (== (+ (Variables|Default|GetLightInt) 1) 4)
    (Variables|Default|SetLightInt 0))
  (CallFunction|SwitchColor (Variables|Default|GetLightInt))
  (if (== (Variables|Default|GetLightInt) (Variables|Default|GetLightOrderNumber))
    (Default|Addto (Variables|Default|GetPuzzleLight_REF))
    ;[1 1 1] Removes on a do once so it doesnt counter out the other lights
    (Utilities|FlowControl|DoOnce false) ; enters at Reset
    (else
      (CallFunction|Remove))))

(event EventBeginPlay
  ;[1 1 1] Set puzzleactor reference
  (bind _outactors (Actor|GetAllActorsOfClass "/Game/BluePrints/NotUsedPuzzle/BP_PuzzleLight.BP_PuzzleLight_C"))
  (Variables|Default|SetPuzzleLight_REF (Utilities|Array|Get(acopy) _outactors)))

(fn ConstructionScript
  (CallFunction|SwitchColor (Variables|Default|GetLightInt)))

(fn SwitchColor
  (params (LightsInt :type Integer))
  (bind _pointlight (Variables|Default|GetPointLight))
  ;[1 1 1] Switch color on point light, based on int
  (switch int LightsInt
    (:0
      (Rendering|Components|Light|SetLightColor _pointlight "(R=0.000000,G=0.050751,B=0.166667,A=1.000000)" true))
    (:1
      (Rendering|Components|Light|SetLightColor _pointlight "(R=0.020109,G=0.192708,B=0.029129,A=1.000000)" true))
    (:2
      (Rendering|Components|Light|SetLightColor _pointlight "(R=0.286458,G=0.000000,B=0.000000,A=1.000000)" true))))