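; BP_KeyCabinet is a cabinet whose door swings open when OpenCabinetDoor is called, per its comment from the tile puzzle.
; A timeline lerps the door's yaw, resetting SquaresActivated and triggering the opening sound at the actor's location on every update.
; An unconnected loop counts lit TilePuzzle squares against nine but never runs.
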(event Custom|OpenCabinetDoor
  ;[1 1 1] When Opencabinet is called from Tilepuzzle, it opens the cabinet door
  (bind _dooropen (Timeline|CabinetDoor Play)
    (:Update
      (Transformation|SetRelativeRotation (Variables|Default|GetDoor) (Math|Rotator|MakeRotator 0.0 0.0 (Math|Float|Lerp 2.7e+02 1.3e+02 _dooropen)) false false)
      (Variables|Default|SetSquaresActivated 0)
      (Audio|PlaySoundatLocation "/Game/Audio/OpenCabinetDoor_Cue.OpenCabinetDoor_Cue" (Transformation|GetActorLocation) "0, 0, 0" 1.0 1.0 0.0 0 0 0 0))))

(fn ConstructionScript)