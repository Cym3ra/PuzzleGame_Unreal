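; BP_TilePuzzle is one tile in a lights-out style puzzle that opens the key cabinet when every tile is lit.
; Interacting flips its own IsOn state and that of each tile in AdjacentPads, playing a click sound.
; It then scans all BP_TilePuzzle actors and calls OpenCabinetDoor on the BP_KeyCabinet found at BeginPlay if all are on.
; Tick swaps the tile material to match IsOn.
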(event EventBeginPlay
  ;[1 1 1] Get reference to BPkeyCabinet to be able to get the custom event OpenCabinet Door
  (bind _returnvalue (Actor|GetActorOfClass "/Game/BluePrints/BP_KeyCabinet.BP_KeyCabinet_C"))
  (Variables|Default|SetKeyCabinet_REF _returnvalue))

(event EventTick
  (params (DeltaSeconds :type Float%20%28single-precision%29))
  (if (Variables|Default|GetisOn?)
    (Rendering|Material|SetMaterial (Variables|Default|GetTile) 0 "/Game/Assets/TileMaterialON_MI.TileMaterialON_MI")
    (else
      (Rendering|Material|SetMaterial (Variables|Default|GetTile) 0 "/Game/Assets/TileMaterialOFF_MI.TileMaterialOFF_MI"))))

(event EventInteract
  (params (Actor :type Actor%20Object%20Reference) (HitResult :type Hit%20Result%20Structure))
  (if (Variables|Default|GetisOn?)
    (Variables|Default|SetisOn? false)
    (else
      (Variables|Default|SetisOn? true)))
  (bind _array_element (Utilities|Array|ForEachLoopwithBreak (Variables|Default|GetAdjacentPads))
    (:LoopBody
      (if (Variables|BP_TilePuzzle_C|GetisOn? _array_element)
        (Variables|BP_TilePuzzle_C|SetisOn? _array_element false)
        (else
          (Variables|BP_TilePuzzle_C|SetisOn? _array_element true)))
      (Audio|PlaySoundatLocation "/Game/Audio/TileClick_Cue.TileClick_Cue" (Transformation|GetActorLocation) "0, 0, 0" 1.0 1.0 0.0 0 0 0 0))
    (:Completed
      ;[1 1 1] Calls the function to check if all tiles are lit, and if they are, open the cabinet door
      (bind _true (CallFunction|CheckAllTiles))
      (if _true
        (Default|OpenCabinetDoor (Variables|Default|GetKeyCabinet_REF))))))

(fn ConstructionScript)

(fn CheckAllTiles
  ;[1 1 1] Gets all the tile actors and checks if they are on, and then returns if they are or not
  (bind _outactors (Actor|GetAllActorsOfClass "BP_TilePuzzle_C"))
  (for _array_element _outactors
    (if (not (Variables|BP_TilePuzzle_C|GetisOn? _array_element))
      (return false)))
  (return true))