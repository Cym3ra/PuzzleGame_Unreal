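; BP_Key is a key pickup that lets the player open the front door.
; On Interact it casts the interacting actor to BP_MyCharacter and sets HasKey to true.
; It then shows the inventory widget's HorizontalBox through a character reference cached on BeginPlay, plays a pickup sound and destroys itself after a short delay.
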(event Custom|DestroyItem
  ;[1 1 1] after 1 sec delay it destroys the key
  (Utilities|FlowControl|Delay 0.1)
  (Actor|DestroyActor))

(event EventBeginPlay
  ;[1 1 1] Get Character reference to get access to the inventory widget
  (bind _returnvalue (Actor|GetActorOfClass "/Game/BluePrints/BP_MyCharacter.BP_MyCharacter_C"))
  (Variables|Default|SetCharacterBP_REF _returnvalue))

(event EventInteract
  (params (Actor :type Actor%20Object%20Reference) (HitResult :type Hit%20Result%20Structure))
  ;[1 1 1] When key is "picked up", it sets the variable haskey in playerBP to true, so that the front door can be opened
  (bind _asbp_my_character (Utilities|Casting|CastToBP_MyCharacter Actor))
  (Variables|/Game/BluePrints/BP_MyCharacter.BP_MyCharacter_C|SethasKey? _asbp_my_character true)
  ;[1 1 1] Gets reference to inventory widget and sets the key to visible on screen
  (Widget|SetVisibility (Variables|/Game/UI/Inventory_Widget.Inventory_Widget_C|GetHorizontalBox (Variables|/Game/BluePrints/BP_MyCharacter.BP_MyCharacter_C|GetInventoryREF (Variables|Default|GetCharacterBP_REF))) "HitTestInvisible")
  (Audio|PlaySoundatLocation "/Game/Audio/PickupKeys_Cue.PickupKeys_Cue" (Transformation|GetActorLocation) "0, 0, 0" 1.0 1.0 0.0 0 0 0 0)
  (CallFunction|DestroyItem))

(fn ConstructionScript)