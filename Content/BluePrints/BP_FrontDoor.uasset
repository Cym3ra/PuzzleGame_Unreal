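; BP_FrontDoor is an interactable front door that opens only if the interacting BP_MyCharacter has the key.
; With the key, the DoorOpen timeline swings the door's yaw open; its Update output also removes the inventory widget and triggers unlock and delayed open sounds.
; Without it, a missing-key widget appears briefly with a locked sound.
; The inventory widget is reached through a character reference cached on BeginPlay.
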(event EventBeginPlay
  ;[1 1 1] get character reference to access inventory widget
  (bind _returnvalue (Actor|GetActorOfClass "/Game/BluePrints/BP_MyCharacter.BP_MyCharacter_C"))
  (Variables|Default|SetCharacterBP_REF _returnvalue))

(event EventInteract
  (params (Actor :type Actor%20Object%20Reference) (HitResult :type Hit%20Result%20Structure))
  (bind _returnvalue (Transformation|GetActorLocation))
  ;[1 1 1] When linetracing it checks if player has key, and if it does it opens the front door
  (bind _asbp_my_character (Utilities|Casting|CastToBP_MyCharacter Actor))
  (if (Variables|/Game/BluePrints/BP_MyCharacter.BP_MyCharacter_C|GethasKey? _asbp_my_character)
    (bind _opendoor (Timeline|DoorOpen PlayFromStart)
      (:Update
        (Transformation|SetRelativeRotation (Variables|Default|GetDoor) (Math|Rotator|MakeRotator 0.0 0.0 (Math|Float|Lerp 0.0 -1e+02 _opendoor)) false false)
        ;[1 1 1] remove inventory widget from screen
        (Widget|RemovefromParent (Variables|/Game/BluePrints/BP_MyCharacter.BP_MyCharacter_C|GetInventoryREF (Variables|Default|GetCharacterBP_REF)))
        (Audio|PlaySoundatLocation "/Game/Audio/UnlockDoor_Cue.UnlockDoor_Cue" _returnvalue "0, 0, 0" 1.0 1.0 0.0 0 0 0 0)
        (Utilities|FlowControl|Delay 0.1)
        (Audio|PlaySoundatLocation "/Game/Audio/OpenDoor_Cue.OpenDoor_Cue" _returnvalue "0, 0, 0" 1.0 1.0 0.0 0 0 0 0)))
    (else
      ;[1 1 1] When trying to open the door without the key, a missing key message will pop up
      (bind _returnvalue_2 (UserInterface|CreateWidget "/Game/UI/MissingKeyWidget.MissingKeyWidget_C"))
      (UserInterface|Viewport|AddtoViewport _returnvalue_2 0)
      (Audio|PlaySoundatLocation "/Game/Audio/DoorLocked_Cue.DoorLocked_Cue" (Transformation|GetActorLocation) "0, 0, 0" 1.0 1.0 0.0 0 0 0 0)
      ;[1 1 1] After 1 sek delay, the message disappears
      (Utilities|FlowControl|Delay 1.0)
      (Widget|RemovefromParent _returnvalue_2))))

(fn ConstructionScript)