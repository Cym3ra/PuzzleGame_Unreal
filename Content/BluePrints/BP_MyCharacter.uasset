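; First-person player character with Enhanced Input move and look, crosshair and inventory widgets, and a toggled pause menu.
; A line trace from the Eyes component sends Interact to any hit actor implementing BPI_Interface.
; Grounded horizontal movement starts a looping footstep sound timer once, which is cleared on stopping or leaving level velocity.
; An event lets movement be disabled entirely.
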(event Custom|PlayFootstepSounds
  ;[1 1 1] Play the footstep sound when character is moving
  (Audio|PlaySoundatLocation "/Game/Audio/FootStep.FootStep" (- (Transformation|GetActorLocation) "0.000000,0.000000,44.000000") "0, 0, 0" 1.0 1.0 0.0 0 0 0 0))

(event Custom|ResetSpeed
  ;[1 1 1] Play the footstep sound when character is moving
  (Utilities|Time|ClearandInvalidateTimerbyHandle (stale Input|EnhancedActionEvents|EnhancedInputActionCustomMove _returnvalue_2))
  (Utilities|FlowControl|DoOnce false) ; enters at Reset
)

(event Custom|StopCharacterMovement
  ;[1 1 1] Stops player movement
  (Pawn|Components|CharacterMovement|DisableMovement (Variables|Character|GetCharacterMovement)))

(event Input|EnhancedActionEvents|EnhancedInputActionCustomMove
  (params (ActionValue :type Vector%202D%20Structure) (ElapsedSeconds :type Float%20%28double-precision%29) (TriggeredSeconds :type Float%20%28double-precision%29) (InputAction :type Input%20Action%20Object%20Reference :default "/Game/Input/CustomMove.CustomMove"))
  (bind _returnvalue (Transformation|GetVelocity))
  ;[1 1 1] Move Character
  (:Triggered
    (Pawn|Input|AddMovementInput (Transformation|GetActorForwardVector) (.y ActionValue) false)
    (Pawn|Input|AddMovementInput (Transformation|GetActorRightVector) (.x ActionValue) false)
    ;[1 1 1] Play the footstep sound when character is moving
    (if (and (Math|Boolean|ORBoolean (< (.x _returnvalue) -0.1) (> (.x _returnvalue) 0.1) (< (.y _returnvalue) -0.1) (> (.y _returnvalue) 0.1)) (== (.z _returnvalue) 0.0))
      (Utilities|FlowControl|DoOnce false :!label _label
        (:Completed
          (bind _returnvalue_2 (Utilities|Time|SetTimerbyEvent (delegate Custom|PlayFootstepSounds) (Variables|Default|GetFootstepInterval) true))))
      (else
        (Utilities|Time|ClearandInvalidateTimerbyHandle _returnvalue_2)
        (goto _label Reset))))
  (:Completed
    (CallFunction|ResetSpeed)))

(event Input|EnhancedActionEvents|EnhancedInputActionCustomInteract
  (params (ActionValue :type Boolean) (ElapsedSeconds :type Float%20%28double-precision%29) (TriggeredSeconds :type Float%20%28double-precision%29) (InputAction :type Input%20Action%20Object%20Reference :default "/Game/Input/CustomInteract.CustomInteract"))
  (bind _eyes (Variables|Default|GetEyes))
  (bind _returnvalue (Transformation|GetWorldLocation _eyes))
  ;[1 1 1] Line trace using left mouse button, if hit and actor uses my BPI Interact, it fires off Interact event in that actor
  (:Triggered
    (bind (_outhit _returnvalue_2) (Collision|LineTraceByChannel _returnvalue (+ _returnvalue (* (Math|Vector|GetForwardVector _eyes) (Variables|Default|GetTraceDistance))) "TraceTypeQuery2" false 0 "None" true "(R=1.000000,G=0.000000,B=0.000000,A=1.000000)" "(R=0.000000,G=1.000000,B=0.000000,A=1.000000)" 1.0))
    (if _returnvalue_2
      (if (Utilities|DoesObjectImplementInterface (.HitActor (Collision|BreakHitResult _outhit)) "/Game/BluePrints/BPI_Interface.BPI_Interface_C")
        (Class|BPIInterface|Interact(Message) (.HitActor (Collision|BreakHitResult _outhit)) self _outhit)))))

(event Input|EnhancedActionEvents|EnhancedInputActionCustomInteract
  (params (ActionValue :type Boolean) (ElapsedSeconds :type Float%20%28double-precision%29) (TriggeredSeconds :type Float%20%28double-precision%29) (InputAction :type Input%20Action%20Object%20Reference :default "/Game/Input/CustomInteract.CustomInteract")))

(event Input|EnhancedActionEvents|EnhancedInputActionCustomLook
  (params (ActionValue :type Vector%202D%20Structure) (ElapsedSeconds :type Float%20%28double-precision%29) (TriggeredSeconds :type Float%20%28double-precision%29) (InputAction :type Input%20Action%20Object%20Reference :default "/Game/Input/CustomLook.CustomLook"))
  ;[1 1 1] Look around using mouse
  (:Triggered
    (Pawn|Input|AddControllerYawInput (.x ActionValue))
    (Pawn|Input|AddControllerPitchInput (.y ActionValue))))

(event Input|EnhancedActionEvents|EnhancedInputActionOpenPausMenu
  (params (ActionValue :type Boolean) (ElapsedSeconds :type Float%20%28double-precision%29) (TriggeredSeconds :type Float%20%28double-precision%29) (InputAction :type Input%20Action%20Object%20Reference :default "/Game/Input/OpenPausMenu.OpenPausMenu"))
  (bind _returnvalue (Game|GetPlayerController 0))
  (bind _returnvalue_2 (Game|GetPlayerController 0))
  ;[1 1 1] When Escape is pressed the first and then every other time it pauses the game. Hides mouse cursor, sets game mode to game and UI, and sets paused to true
  (:Triggered
    (Utilities|FlowControl|FlipFlop
      (:A
        (bind _returnvalue_3 (UserInterface|CreateWidget "/Game/UI/PausMenu.PausMenu_C"))
        (UserInterface|Viewport|AddtoViewport _returnvalue_3 0)
        (Game|SetGamePaused true)
        (Input|SetInputModeGameandUI _returnvalue_2 0 "DoNotLock" true false)
        (Variables|/Script/Engine.PlayerController|SetbShowMouseCursor _returnvalue_2 true))
      (:B
        ;[1 1 1] When Button is pressed again it unpauses the game and sets mouse and game mode back to game
        (Widget|RemovefromParent _returnvalue_3)
        (Input|SetInputModeGameOnly _returnvalue false)
        (Variables|/Script/Engine.PlayerController|SetbShowMouseCursor _returnvalue false)
        (Game|SetGamePaused false)))))

(event EventBeginPlay
  ;[1 1 1] Add Input (IMC) to player controller character
  (bind _asplayer_controller (Utilities|Casting|CastToPlayerController (Pawn|GetController)))
  (Input|AddMappingContext (PlayerController|LocalPlayerSubsystems|GetEnhancedInputLocalPlayerSubsystem _asplayer_controller) "/Game/Input/Custom_IMC.Custom_IMC" 0 "(bIgnoreAllPressedKeysUntilRelease=True,bForceImmediately=False)")
  ;[1 1 1] Creates the crosshair dot widget on screen
  (bind _returnvalue (UserInterface|CreateWidget "/Game/BluePrints/InteractDot_Widget.InteractDot_Widget_C"))
  (bind _output_get (Variables|Default|SetInteractDot_Ref _returnvalue))
  (UserInterface|Viewport|AddtoViewport _output_get 0)
  ;[1 1 1] Add inventory widget to screen
  (bind _returnvalue_2 (UserInterface|CreateWidget "/Game/UI/Inventory_Widget.Inventory_Widget_C"))
  (bind _output_get_2 (Variables|Default|SetInventoryREF _returnvalue_2))
  (UserInterface|Viewport|AddtoViewport _output_get_2 0))

(event Collision|EventActorBeginOverlap
  (params (OtherActor :type Actor%20Object%20Reference)))

(event EventTick
  (params (DeltaSeconds :type Float%20%28single-precision%29)))

(fn ConstructionScript)