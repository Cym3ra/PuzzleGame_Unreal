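; Interactable lamp switch actor that cycles its point light through white, blue, red and green.
; Each Interact event increments ColorIndex, wraps it to zero after the last color, then plays a click sound at the actor's location.
; UpdateLightColor maps the index to a hard-coded color on the PointLight, and only runs on interaction.
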(event EventBeginPlay)

(event Collision|EventActorBeginOverlap
  (params (OtherActor :type Actor%20Object%20Reference)))

(event EventTick
  (params (DeltaSeconds :type Float%20%28single-precision%29)))

(event EventInteract
  (params (Actor :type Actor%20Object%20Reference) (HitResult :type Hit%20Result%20Structure))
  (bind _result (Math|Integer|IncrementInt (Variables|Default|GetColorIndex))
    (:%20%20
      (if (<= _result 3)
        _
        (else
          (Variables|Default|SetColorIndex 0)))
      (CallFunction|UpdateLightColor)
      (Audio|PlaySoundatLocation "/Game/Audio/LampClick_Cue.LampClick_Cue" (Transformation|GetActorLocation) "0, 0, 0" 1.0 1.0 0.0 0 0 0 0))))

(fn ConstructionScript)

(fn UpdateLightColor
  (switch int (Variables|Default|GetColorIndex)
    (:0
      (Rendering|Components|Light|SetLightColor (Variables|Default|GetPointLight) "(R=1.000000,G=1.000000,B=1.000000,A=1.000000)" true))
    (:1
      (Rendering|Components|Light|SetLightColor (Variables|Default|GetPointLight) "(R=0.000000,G=0.017805,B=0.432292,A=1.000000)" true))
    (:2
      (Rendering|Components|Light|SetLightColor (Variables|Default|GetPointLight) "(R=0.359375,G=0.002984,B=0.000000,A=1.000000)" true))
    (:3
      (Rendering|Components|Light|SetLightColor (Variables|Default|GetPointLight) "(R=0.000424,G=0.223958,B=0.000000,A=1.000000)" true))))