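; Symbol puzzle actor with four colored turntables and a check button that opens a linked door when the symbol combination is correct.
; Interact reads the hit component's tag to rotate a turntable a quarter turn via timeline, with CanRotate blocking overlapping input.
; The check button converts each table's yaw into an enum, compares that array against CorrectAnswer, then plays success or failure button animation and sound, calling Interact on DoorToOpen upon success.
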(event Custom|RotateSymbols
  ;[1 1 1] Event to rotate the turntable on target
  (bind (_startrot _endrot) (CallFunction|SymbolRotate))
  (bind _alpha (Timeline|RotateTL PlayFromStart)
    (:Update
      (Transformation|SetRelativeRotation (Variables|Default|GetSymbolToRotate) (Math|Rotator|Lerp(Rotator) _startrot _endrot _alpha) false false))
    (:Finished
      (Variables|Default|SetcanRotate? true))))

(event EventBeginPlay
  (bind _returnvalue (Actor|GetActorOfClass "/Game/BluePrints/BP_MyCharacter.BP_MyCharacter_C"))
  (Variables|Default|SetCharacter_REF _returnvalue))

(event EventInteract
  (params (Actor :type Actor%20Object%20Reference) (HitResult :type Hit%20Result%20Structure))
  (bind _button (Variables|Default|GetButton))
  ;[1 1 1] On event Interact, check which tag is the target and call event Rotate on that target( the boolean check is to make sure a target isn't already rotating, if it is the new target won't rotate)
  (if (Variables|Default|GetcanRotate?)
    (Variables|Default|SetcanRotate? false)
    (switch name (Utilities|Array|Get(acopy) (Variables|/Script/Engine.ActorComponent|GetComponentTags (.HitComponent (Collision|BreakHitResult HitResult))))
      (:Blue
        (Variables|Default|SetSymbolToRotate (Variables|Default|GetBlueTurnTable))
        (CallFunction|RotateSymbols :!label _label)
        (Audio|PlaySoundatLocation "/Game/Audio/RotatingStone_Cue.RotatingStone_Cue" (Transformation|GetActorLocation) "0, 0, 0" 1.0 1.0 0.0 0 0 0 0))
      (:Green
        (Variables|Default|SetSymbolToRotate (Variables|Default|GetGreenTurnTable))
        (goto _label))
      (:Red
        (Variables|Default|SetSymbolToRotate (Variables|Default|GetRedTurnTable))
        (goto _label))
      (:Yellow
        (Variables|Default|SetSymbolToRotate (Variables|Default|GetYellowTurnTable))
        (goto _label))
      (:CheckButton
        (CallFunction|SetupPlayerAnswer)
        (Utilities|FlowControl|Delay 0.2)
        (bind _iswinner_ (CallFunction|CheckAnswer))
        (if _iswinner_
          (bind _buttonpressed (Timeline|ButtonPress PlayFromStart)
            (:Update
              (Transformation|SetRelativeLocation _button _buttonpressed false false)
              (Rendering|Material|SetMaterial _button 0 "/Game/Assets/MasterMaterial_MI_Two.MasterMaterial_MI_Two")
              (Audio|PlaySoundatLocation "/Game/Audio/Success_Cue.Success_Cue" (Transformation|GetWorldLocation (Variables|Default|GetInteractButton)) "0, 0, 0" 1.0 1.0 0.0 0 0 0 0)
              (Default|Interact (Variables|Default|GetDoorToOpen) self))
            (:Finished
              (Rendering|Material|SetMaterial _button 0 "/Game/StarterContent/Materials/M_Basic_Wall.M_Basic_Wall")))
          (else
            (bind _pressfailed (Timeline|ButtonFail PlayFromStart)
              (:Update
                (Transformation|SetRelativeLocation (Variables|Default|GetButton) _pressfailed false false)
                (Audio|PlaySoundatLocation "/Game/Audio/Error_Cue.Error_Cue" (Transformation|GetWorldLocation (Variables|/Script/Engine.Actor|GetRootComponent (Variables|Default|GetCharacter_REF))) "0, 0, 0" 0.3 0.8 0.0 0 0 0 0)))))))))

(fn ConstructionScript)

(fn SymbolRotate
  (bind _symboltorotate (Variables|Default|GetSymbolToRotate))
  (bind _relativerotation (Variables|/Script/Engine.SceneComponent|GetRelativeRotation _symboltorotate))
  (bind _returnvalue (+ (.yaw _relativerotation) 9e+01))
  ;[1 1 1] Checks the start rotation of target, and if it tries to go over 360, puts it back to 0 again
  (LocalVariables|SetStartRotation (Math|Rotator|MakeRotator 0.0 0.0 (.yaw _relativerotation)))
  (LocalVariables|SetEndRotation (Math|Rotator|MakeRotator 0.0 0.0 (Math|Float|SelectFloat 0.0 _returnvalue (> _returnvalue 3.6e+02))))
  (return (LocalVariables|GetStartRotation) (LocalVariables|GetEndRotation)))

(fn GetSymbolAnswerbyRotation
  (params (PillarRot :type Rotator))
  (if (Utilities|Operators|EqualEqual :A PillarRot :ErrorTolerance 1.0)
    (LocalVariables|SetAnswer "NewEnumerator0")
    (elif (Utilities|Operators|EqualEqual PillarRot "0.000000,90.000000,0.000000" 1.0)
      (LocalVariables|SetAnswer "NewEnumerator1")
      (elif (Utilities|Operators|EqualEqual PillarRot "0.000000,-90.000000,0.000000" 1.0)
        (LocalVariables|SetAnswer "NewEnumerator3")
        (else
          (LocalVariables|SetAnswer "NewEnumerator2")))))
  (return (LocalVariables|GetAnswer)))

(fn SetupPlayerAnswer
  (Utilities|FlowControl|Sequence
    (:then_0
      (bind _pillaranswer (CallFunction|GetSymbolAnswerbyRotation (Variables|/Script/Engine.SceneComponent|GetRelativeRotation (Variables|Default|GetGreenTurnTable))))
      (Utilities|Array|SetArrayElem (Variables|Default|GetPlayerAnswer) 0 _pillaranswer))
    (:then_1
      (bind _pillaranswer_2 (CallFunction|GetSymbolAnswerbyRotation (Variables|/Script/Engine.SceneComponent|GetRelativeRotation (Variables|Default|GetBlueTurnTable))))
      (Utilities|Array|SetArrayElem (Variables|Default|GetPlayerAnswer) 1 _pillaranswer_2))
    (:then_2
      (bind _pillaranswer_3 (CallFunction|GetSymbolAnswerbyRotation (Variables|/Script/Engine.SceneComponent|GetRelativeRotation (Variables|Default|GetRedTurnTable))))
      (Utilities|Array|SetArrayElem (Variables|Default|GetPlayerAnswer) 2 _pillaranswer_3))
    (:then_3
      (bind _pillaranswer_4 (CallFunction|GetSymbolAnswerbyRotation (Variables|/Script/Engine.SceneComponent|GetRelativeRotation (Variables|Default|GetYellowTurnTable))))
      (Utilities|Array|SetArrayElem (Variables|Default|GetPlayerAnswer) 3 _pillaranswer_4))))

(fn CheckAnswer
  (bind (_array_element _array_index) (Utilities|Array|ForEachLoopwithBreak (Variables|Default|GetCorrectAnswer) :!label _label)
    (:LoopBody
      (if (not (Utilities|Enum|Equal(Enum) _array_element (Utilities|Array|Get(acopy) (Variables|Default|GetPlayerAnswer) _array_index)))
        (LocalVariables|SetWinner? false)
        (goto _label Break)))
    (:Completed
      (Variables|Default|SetcanRotate? true)
      (return (LocalVariables|GetWinner?)))))